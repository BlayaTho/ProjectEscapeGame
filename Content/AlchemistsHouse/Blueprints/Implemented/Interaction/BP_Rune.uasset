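; BP_Rune is an interactable rune, revealed by power vision, that removes its linked rune door.
; The PowerVision event toggles the Niagara effect's visibility and the box's query-only collision together.
; Interaction runs once via DoOnce, destroying RuneDoor, disabling the box and hiding the effect.
; The rune actor itself persists, so later PowerVision activations still show the effect and re-enable collision.
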(event EventInteraction
  (params (CamVector :type Vector :default "0, 0, 0"))
  (Utilities|FlowControl|DoOnce false
    (:Completed
      (Actor|DestroyActor (Variables|Default|GetRuneDoor))
      (Collision|SetCollisionEnabled (Variables|Default|GetBox) "NoCollision")
      (Development|SetHiddeninGame (Variables|Default|GetNiagara) true false))))

(event EventPowerVision
  (params (VisionON :type Boolean))
  (if VisionON
    (Collision|SetCollisionEnabled (Variables|Default|GetBox) "QueryOnly")
    (Development|SetHiddeninGame (Variables|Default|GetNiagara) false false)
    (else
      (Collision|SetCollisionEnabled (Variables|Default|GetBox) "NoCollision")
      (Development|SetHiddeninGame (Variables|Default|GetNiagara) true false))))

(fn ConstructionScript)