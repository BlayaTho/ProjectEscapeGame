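; BP_Candle_5 is an interactable candle in an ordered snuffing puzzle tied to a bookcase.
; On interaction it casts BougieAvant to BP_Candle_4 and hides its own flame, setting IsShut, only if that candle is already out.
; Otherwise it calls WrongAnswer on the bookcase.
; ResetAllBougie shows the flame again and clears IsShut.
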(event EventResetAllBougie
  (Development|SetHiddeninGame (Variables|Default|GetFlame) false false)
  (Variables|Default|SetisShut false))

(event EventInteraction
  (params (CamVector :type Vector :default "0, 0, 0"))
  (bind _asbp_candle_4 (Utilities|Casting|CastToBP_Candle_4 (Variables|Default|GetBougie%20Avant)))
  (if (Variables|/Game/AlchemistsHouse/Blueprints/Implemented/Interaction/cozy/BP_Candle_4.BP_Candle_4_C|GetisShut _asbp_candle_4)
    (Development|SetHiddeninGame (Variables|Default|GetFlame) true false)
    (Variables|Default|SetisShut true)
    (else
      (Default|WrongAnswer (Variables|Default|GetBookcaseRef)))))

(fn ConstructionScript)