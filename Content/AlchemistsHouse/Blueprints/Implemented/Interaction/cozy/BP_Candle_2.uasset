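; BP_Candle_2 is an interactable candle that forms a step in an ordered candle-snuffing puzzle tied to a bookcase.
; On interaction it casts its preceding-candle reference to BP_Candle_1 and, if that candle is out, hides its own flame and marks itself shut.
; Otherwise it reports a wrong answer to the bookcase.
; A reset event relights the flame and clears the shut state.
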(event EventResetAllBougie
  (Development|SetHiddeninGame (Variables|Default|GetFlame) false false)
  (Variables|Default|SetisShut false))

(event EventInteraction
  (params (CamVector :type Vector :default "0, 0, 0"))
  (bind _asbp_candle_1 (Utilities|Casting|CastToBP_Candle_1 (Variables|Default|GetbougieAvant)))
  (if (Variables|/Game/AlchemistsHouse/Blueprints/Implemented/Interaction/cozy/BP_Candle_1.BP_Candle_1_C|GetisShut _asbp_candle_1)
    (Development|SetHiddeninGame (Variables|Default|GetFlame) true false)
    (Variables|Default|SetisShut true)
    (else
      (Default|WrongAnswer (Variables|Default|GetBookcaseRef)))))

(fn ConstructionScript)