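; BP_Candle_6 is an interactable candle in an ordered extinguishing puzzle that moves a bookcase.
; On interaction it checks that the preceding BP_Candle_5, referenced through BougieAvant, is shut, then hides its own flame and triggers the bookcase's EventMove only once.
; If that candle is still lit, it reports WrongAnswer to the bookcase.
; ResetAll shows the flame again and clears its shut state.
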(event EventResetAll
  (Development|SetHiddeninGame (Variables|Default|GetFlame) false false)
  (Variables|Default|SetisShut false))

(event EventInteraction
  (params (CamVector :type Vector :default "0, 0, 0"))
  (bind _asbp_candle_5 (Utilities|Casting|CastToBP_Candle_5 (Variables|Default|GetBougie%20Avant)))
  (if (Variables|/Game/AlchemistsHouse/Blueprints/Implemented/Interaction/cozy/BP_Candle_5.BP_Candle_5_C|GetisShut _asbp_candle_5)
    (Development|SetHiddeninGame (Variables|Default|GetFlame) true false)
    (Variables|Default|SetisShut true)
    (Utilities|FlowControl|DoOnce false
      (:Completed
        (Default|EventMove (Variables|Default|GetBookcaseRef))))
    (else
      (Default|WrongAnswer (Variables|Default|GetBookcaseRef)))))

(fn ConstructionScript)