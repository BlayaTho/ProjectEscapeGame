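; BP_BookRed is the red book in an Alchemist's House bookcase puzzle, visible and detectable only during power vision.
; PowerVision toggles the query collision of its Box and the visibility of its NSBookRed effect.
; Interaction fires once through a DoOnce, flags BookTriggered on the referenced bookcase, pauses the effect, calls WrongAnswer and prints a French mechanism-noise message.
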(event EventPowerVision
  (params (VisionON :type Boolean))
  (bind _ns_bookred (Variables|Default|GetNS_BookRed))
  (bind _box (Variables|Default|GetBox))
  (if VisionON
    (Collision|SetCollisionEnabled _box "QueryOnly")
    (Development|SetHiddeninGame _ns_bookred false false)
    (else
      (Collision|SetCollisionEnabled _box "NoCollision")
      (Development|SetHiddeninGame _ns_bookred true false))))

(event EventInteraction
  (params (CamVector :type Vector :default "0, 0, 0"))
  (Utilities|FlowControl|DoOnce false
    (:Completed
      (Variables|/Game/AlchemistsHouse/Blueprints/Implemented/Interaction/cozy/BP_Bookcase.BP_Bookcase_C|SetBookTriggered (Variables|Default|GetBookcaseREF) true)
      (Class|NiagaraComponent|SetPaused (Variables|Default|GetNS_BookRed) true)
      (Default|WrongAnswer (Variables|Default|GetBookcaseREF))
      (Development|PrintString "*J'entend un bruit* Un mecanisme a été activé" true true "(R=1.000000,G=1.000000,B=1.000000,A=1.000000)" 4.0))))

(fn ConstructionScript)