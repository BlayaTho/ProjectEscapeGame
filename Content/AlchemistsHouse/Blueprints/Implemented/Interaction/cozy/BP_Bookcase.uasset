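; Bookcase in the Alchemist's House that slides aside with a camera shake and handles wrong answers in a candle interaction.
; EventMove plays a world camera shake, then a timeline lerps the root's X from its current position to a hardcoded world coordinate.
; WrongAnswer calls ResetAllMessage on every candle in AllBougie, but only if BookTriggered is set.
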(event Custom|EventMove
  (bind _returnvalue (Transformation|GetActorLocation))
  (Camera|PlayWorldCameraShake "/Game/AlchemistsHouse/Blueprints/Implemented/BP_CameraShake.BP_CameraShake_C" (Transformation|GetWorldLocation (Variables|Default|GetSharedRoot)) 0.0 1e+03)
  (bind _output_get (Variables|Default|SetInitialLocation (Transformation|GetWorldLocation (Variables|Default|GetSharedRoot))))
  (bind _lerp (Timeline|Movement PlayFromStart)
    (:Update
      (Transformation|SetWorldLocation (Variables|Default|GetSharedRoot) (Math|Vector|MakeVector (Math|Float|Lerp (.x _output_get) -944.0 _lerp) (.y _returnvalue) (.z _returnvalue)) false false))))

(event Custom|WrongAnswer
  (if (Variables|Default|GetBookTriggered)
    (for _array_element (Variables|Default|GetAllBougie)
      (Class|BPIInteraction|ResetAll(Message) _array_element))))

(fn ConstructionScript)