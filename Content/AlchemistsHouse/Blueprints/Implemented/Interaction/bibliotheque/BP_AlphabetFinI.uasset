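; BP_AlphabetFinI is an interactable letter I in the library (bibliotheque) word puzzle tied to a chest.
; On interaction, it marks itself Touched only if the referenced letter L has already been touched, enforcing the spelling order.
; An out-of-order or repeated touch calls WrongWord on the chest, and ResetAll clears the Touched flag.
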(event EventInteraction
  (params (CamVector :type Vector :default "0, 0, 0"))
  (if (Variables|Default|GetTouched)
    (Default|WrongWord (Variables|Default|GetChestREF) :!label _label)
    (else
      (bind _asbp_alphabet_fin_l (Utilities|Casting|CastToBP_AlphabetFinL (Variables|Default|GetLREF)))
      (if (Variables|/Game/AlchemistsHouse/Blueprints/Implemented/Interaction/bibliotheque/BP_AlphabetFinL.BP_AlphabetFinL_C|GetTouched _asbp_alphabet_fin_l)
        (Variables|Default|SetTouched true)
        (else
          (goto _label))))))

(event EventResetAll
  (Variables|Default|SetTouched false))

(fn ConstructionScript)