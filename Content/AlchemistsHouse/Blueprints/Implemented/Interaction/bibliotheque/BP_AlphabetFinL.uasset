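; BP_AlphabetFinL is an interactable letter in the Alchemist's House library word puzzle, apparently the L that must follow A.
; Interaction marks it Touched only if the referenced BP_AlphabetFinA is already touched.
; Repeating it or touching it out of order calls WrongWord on the chest reference.
; ResetAll clears the Touched flag.
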(event EventResetAll
  (Variables|Default|SetTouched false))

(event EventInteraction
  (params (CamVector :type Vector :default "0, 0, 0"))
  (if (Variables|Default|GetTouched)
    (Default|WrongWord (Variables|Default|GetChestREF) :!label _label)
    (else
      (bind _asbp_alphabet_fin_a (Utilities|Casting|CastToBP_AlphabetFinA (Variables|Default|GetAREF)))
      (if (Variables|/Game/AlchemistsHouse/Blueprints/Implemented/Interaction/bibliotheque/BP_AlphabetFinA.BP_AlphabetFinA_C|GetTouched _asbp_alphabet_fin_a)
        (Variables|Default|SetTouched true)
        (else
          (goto _label))))))

(fn ConstructionScript)