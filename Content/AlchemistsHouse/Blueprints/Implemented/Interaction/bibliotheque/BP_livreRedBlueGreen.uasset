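; Interactive library book (red/blue/green) that triggers a linked bookcase puzzle element once.
; Interaction either calls the bookcase's move event or, for the second book, runs a timeline that scales up a referenced stand while calling CloseBookcase on each update.
; PowerVision toggles the Niagara effect and, unless flagged non-interactive, enables query-only collision so the book responds only while vision is on.
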(event EventInteraction
  (params (CamVector :type Vector :default "0, 0, 0"))
  (if (not (Variables|Default|GetisNoInteractif))
    (if (Variables|Default|GetisBook2)
      (Utilities|FlowControl|DoOnce false
        (:Completed
          (bind _lerp (Timeline|Timeline PlayFromStart)
            (:Update
              (Transformation|SetActorScale3D (Variables|Default|GetstandRef) (Math|Vector|MakeVector (Math|Float|Lerp 0.2 1.0 _lerp) (Math|Float|Lerp 0.2 1.0 _lerp) (Math|Float|Lerp 0.2 1.0 _lerp)))
              (Default|CloseBookcase (Variables|Default|GetBookcase2))))))
      (else
        (Utilities|FlowControl|DoOnce false
          (:Completed
            (Default|EventMove (Variables|Default|GetBookcase2))))))))

(event EventPowerVision
  (params (VisionON :type Boolean))
  (bind _staticmesh (Variables|Default|GetStaticMesh))
  (if VisionON
    (if (Variables|Default|GetisNoInteractif)
      _
      (else
        (Collision|SetCollisionEnabled _staticmesh "QueryOnly")))
    (Development|SetHiddeninGame (Variables|Default|GetNiagara) false false)
    (else
      (if (Variables|Default|GetisNoInteractif)
        _
        (else
          (Collision|SetCollisionEnabled _staticmesh "NoCollision")))
      (Development|SetHiddeninGame (Variables|Default|GetNiagara) true false))))

(fn ConstructionScript)