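; Teleporting apple pickup that moves around the level and counts toward the player's recipe fruit total.
; On BeginPlay it caches TargetPoints tagged "apple"; DebutTeleport activates it and starts a looping timer.
; Each tick of that timer shuffles the points, picks one other than its current position, and glides there through a Timeline lerp.
; Interaction while active increments NbrFruitRecette on BP_FirstPersonCharacter and destroys the apple.
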(event Custom|DebutTeleport
  (Variables|Default|SetIsActive true)
  (Utilities|Time|SetTimerbyEvent (delegate Custom|Teleportation) 2.0 true))

(event Custom|Teleportation
  (bind _targetteleport (Variables|Default|GetTargetTeleport))
  (bind _output (Utilities|Array|Get(acopy) _targetteleport))
  (bind _returnvalue (Transformation|GetActorLocation _output))
  (Utilities|Array|Shuffle _targetteleport)
  (if (Utilities|Operators|EqualEqual _returnvalue (Transformation|GetActorLocation) 0.0)
    (Variables|Default|SetFinalLocation (Transformation|GetActorLocation (Utilities|Array|Get(acopy) (Variables|Default|GetTargetTeleport) 1)))
    (bind _lerp (Timeline|Timeline PlayFromStart)
      (:Update
        (Transformation|SetActorLocation (Math|Vector|Lerp(Vector) (Transformation|GetActorLocation) (Variables|Default|GetFinalLocation) _lerp) false false)))
    (else
      (Variables|Default|SetFinalLocation _returnvalue)
      (Timeline|Timeline PlayFromStart))))

(event EventInteraction
  (params (CamVector :type Vector :default "0, 0, 0"))
  (if (Variables|Default|GetIsActive)
    (bind _asbp_first_person_character (Utilities|Casting|CastToBP_FirstPersonCharacter (Game|GetPlayerCharacter 0)))
    (bind _result (Math|Integer|IncrementInt (Variables|/Game/AlchemistsHouse/Blueprints/Implemented/Character/BP_FirstPersonCharacter.BP_FirstPersonCharacter_C|GetNbrFruitRecette _asbp_first_person_character))
      (:%20%20
        (Variables|/Game/AlchemistsHouse/Blueprints/Implemented/Character/BP_FirstPersonCharacter.BP_FirstPersonCharacter_C|SetNbrFruitRecette _asbp_first_person_character _result)
        (Actor|DestroyActor)))))

(event EventBeginPlay
  (bind _outactors (Actor|GetAllActorsOfClasswithTag "/Script/Engine.TargetPoint" "apple"))
  (Variables|Default|SetTargetTeleport _outactors))

(fn ConstructionScript)