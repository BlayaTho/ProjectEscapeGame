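; BP_Egg is an interactable egg pickup for a cuisine recipe in the Alchemist's House.
; When interacted with while active, it increments the first-person character's NbrFruitRecette counter and destroys itself.
; While inactive, it instead sends the character an objective text remarking on the egg under the table.
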(event EventInteraction
  (params (CamVector :type Vector :default "0, 0, 0"))
  (if (Variables|Default|GetisActive)
    (bind _asbp_first_person_character (Utilities|Casting|CastToBP_FirstPersonCharacter (Game|GetPlayerCharacter 0)))
    (bind _result (Math|Integer|IncrementInt (Variables|/Game/AlchemistsHouse/Blueprints/Implemented/Character/BP_FirstPersonCharacter.BP_FirstPersonCharacter_C|GetNbrFruitRecette _asbp_first_person_character))
      (:%20%20
        (Variables|/Game/AlchemistsHouse/Blueprints/Implemented/Character/BP_FirstPersonCharacter.BP_FirstPersonCharacter_C|SetNbrFruitRecette _asbp_first_person_character _result)
        (Actor|DestroyActor)))
    (else
      (bind _asbp_first_person_character_2 (Utilities|Casting|CastToBP_FirstPersonCharacter (Game|GetPlayerCharacter 0)))
      (Default|NewObjectif _asbp_first_person_character_2 "What's an egg doing under the table ?" false))))

(fn ConstructionScript)