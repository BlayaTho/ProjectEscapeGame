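; BP_levier is an interactable lever in the Alchemist's House that starts a timed staircase movement at the house entrance.
; Interaction spins the mesh on one timeline, slides the referenced staircase on another and prints French hint text.
; After a 13-second countdown both timelines reverse and the DoOnce re-arms, unless Finish is set.
; The first-person character overlapping the Box sets Finish, playing the staircase timeline forward if needed and disabling further interaction.
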(event OnComponentBeginOverlap(Box)
  (params (OverlappedComponent :type Primitive%20Component%20Object%20Reference) (OtherActor :type Actor%20Object%20Reference) (OtherComp :type Primitive%20Component%20Object%20Reference) (OtherBodyIndex :type Integer) (bFromSweep :type Boolean) (SweepResult :type Hit%20Result%20Structure%20%28by%20ref%29))
  (Utilities|Casting|CastToBP_FirstPersonCharacter OtherActor)
  (if (!= (.x (Transformation|GetActorLocation (Variables|Default|GetEscalierREF))) 229.0)
    (Utilities|FlowControl|Sequence
      (:then_0
        (bind _lerp (Timeline|Timeline Play)
          (:Update
            (Transformation|SetActorLocation (Variables|Default|GetEscalierREF) (Math|Vector|MakeVector (Math|Float|Lerp 473.0 229.0 _lerp) 3457.0 1e+02) false false)
            (Utilities|FlowControl|DoOnce false
              (:Completed
                (Utilities|FlowControl|Delay 13.0)
                (if (not (Variables|Default|Getfinish))
                  (Utilities|FlowControl|Sequence
                    (:then_0
                      (Timeline|Timeline ReverseFromEnd))
                    (:then_1
                      (Development|PrintString "Le compte à rebours s'est éteint" true true "(R=1.000000,G=1.000000,B=1.000000,A=1.000000)" 4.0)
                      (bind _lerp_2 (Timeline|Timeline_0 ReverseFromEnd)
                        (:Update
                          (Transformation|SetRelativeRotation (Variables|Default|GetStaticMesh) (Math|Rotator|MakeRotator 0.0 (Math|Float|Lerp 0.0 -4.5e+02 _lerp_2) -1.8e+02) false false))))
                    (:then_2
                      (Utilities|FlowControl|DoOnce false) ; enters at Reset
                    ))))))))
      (:then_1
        (Variables|Default|Setfinish true :!label _label)))
    (else
      (goto _label))))

(event Custom|RotateWell
  (bind _lerp (Timeline|Timeline_0 PlayFromStart)
    (:Update
      (Transformation|SetRelativeRotation (Variables|Default|GetStaticMesh) (Math|Rotator|MakeRotator 0.0 (Math|Float|Lerp 0.0 -4.5e+02 _lerp) -1.8e+02) false false))))

(event EventInteraction
  (params (CamVector :type Vector :default "0, 0, 0"))
  (if (not (Variables|Default|Getfinish))
    (Utilities|FlowControl|DoOnce false :!label _label
      (:Completed
        (CallFunction|RotateWell)
        (Development|PrintString "J'entend comme un compte à rebours et quelque chose bouger à l'entrée de la maison." true true "(R=1.000000,G=1.000000,B=1.000000,A=1.000000)" 12.0)
        (Utilities|FlowControl|Sequence
          (:then_0
            (goto _label_2 Reset))
          (:then_1
            (bind _lerp (Timeline|Timeline PlayFromStart)
              (:Update
                (Transformation|SetActorLocation (Variables|Default|GetEscalierREF) (Math|Vector|MakeVector (Math|Float|Lerp 473.0 229.0 _lerp) 3457.0 1e+02) false false)
                (Utilities|FlowControl|DoOnce false :!label _label_2
                  (:Completed
                    (Utilities|FlowControl|Delay 13.0)
                    (if (not (Variables|Default|Getfinish))
                      (Utilities|FlowControl|Sequence
                        (:then_0
                          (Timeline|Timeline ReverseFromEnd))
                        (:then_1
                          (Development|PrintString "Le compte à rebours s'est éteint" true true "(R=1.000000,G=1.000000,B=1.000000,A=1.000000)" 4.0)
                          (bind _lerp_2 (Timeline|Timeline_0 ReverseFromEnd)
                            (:Update
                              (Transformation|SetRelativeRotation (Variables|Default|GetStaticMesh) (Math|Rotator|MakeRotator 0.0 (Math|Float|Lerp 0.0 -4.5e+02 _lerp_2) -1.8e+02) false false))))
                        (:then_2
                          (goto _label Reset))))))))))))))

(fn ConstructionScript)