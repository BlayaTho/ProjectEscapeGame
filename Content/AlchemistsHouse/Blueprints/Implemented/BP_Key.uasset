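; BP_Key is a pickup key that the player collects through an Interaction event, then destroys itself.
; An IsKey1 flag picks which key flag it sets on the BP_FirstPersonCharacter.
; The first key also unlocks its referenced BPDoor and immediately triggers that door's Interaction, while the second only records possession on the character.
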(event EventInteraction
  (params (CamVector :type Vector :default "0, 0, 0"))
  (bind _bp_door (Variables|Default|GetBP_Door))
  (Utilities|FlowControl|Sequence
    (:then_0
      (bind _asbp_first_person_character (Utilities|Casting|CastToBP_FirstPersonCharacter (Game|GetPlayerCharacter 0)))
      (if (Variables|Default|GetIsKey1)
        (Variables|/Game/AlchemistsHouse/Blueprints/Implemented/BP_FirstPersonCharacter.BP_FirstPersonCharacter_C|SetKey1 _asbp_first_person_character true)
        (Variables|/Game/AlchemistsHouse/Blueprints/Implemented/BP_Door.BP_Door_C|SetCanOpen _bp_door true)
        (Default|Interaction _bp_door "0, 0, 0")
        (else
          (Variables|/Game/AlchemistsHouse/Blueprints/Implemented/BP_FirstPersonCharacter.BP_FirstPersonCharacter_C|SetKey2 _asbp_first_person_character true))))
    (:then_1
      (Actor|DestroyActor))))

(fn ConstructionScript)