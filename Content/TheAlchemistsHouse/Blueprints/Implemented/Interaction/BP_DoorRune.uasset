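; Double door in The Alchemist's House that opens or closes on interaction once the first-person character holds exactly four 1F runes.
; A FlipFlop plays or reverses a timeline, rate-scaled by Duration, that yaws both leaves in opposite directions.
; Before opening, the camera vector is compared to the aperture's right vector to pick the swing direction.
; The IsOpening guard clears on the timeline's Update rather than on Finished.
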(event EventBeginPlay
  (Components|Timeline|SetPlayRate (Variables|Default|GetMovementDoor) (/ 1.0 (Variables|OpeningSystem|GetDuration))))

(event EventInteraction
  (params (CamVector :type Vector :default "0, 0, 0"))
  (bind _asbp_first_person_character (Utilities|Casting|CastToBP_FirstPersonCharacter (Game|GetPlayerCharacter 0)))
  (if (== (Variables|/Game/TheAlchemistsHouse/Blueprints/Implemented/Character/BP_FirstPersonCharacter.BP_FirstPersonCharacter_C|GetNbrRunes1F _asbp_first_person_character) 4)
    (if (not (Variables|Default|GetIsOpening))
      (if (Variables|Default|GetIsOpen)
        _
        (elif (Utilities|Operators|EqualEqual CamVector (Math|Vector|GetRightVector (Variables|Default|GetSM_Door_aperture)) 1.0)
          (Variables|OpeningSystem|SetRotationAngle (* (Variables|OpeningSystem|GetRotationAngle) -1.0))
          (else
            (Variables|OpeningSystem|SetRotationAngle (Math|Float|Absolute(Float) (Variables|OpeningSystem|GetRotationAngle))))))
      (Utilities|FlowControl|FlipFlop
        (:A
          (Variables|Default|SetIsOpening true)
          (Variables|Default|SetIsOpen true)
          (bind _newtrack_0 (Timeline|MovementDoor Play)
            (:Update
              (Transformation|SetRelativeRotation (Variables|Default|GetSM_DoorL) (Math|Rotator|MakeRotator 0.0 0.0 (* (* _newtrack_0 (Variables|OpeningSystem|GetRotationAngle)) -1.0)) false false)
              (Transformation|SetRelativeRotation (Variables|Default|GetSM_DoorR) (Math|Rotator|MakeRotator 0.0 0.0 (* _newtrack_0 (Variables|OpeningSystem|GetRotationAngle))) false false)
              (Variables|Default|SetIsOpening false))))
        (:B
          (Variables|Default|SetIsOpening true)
          (Variables|Default|SetIsOpen false)
          (Timeline|MovementDoor Reverse))))))

(fn ConstructionScript)