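; BP_Candle_1 is an interactable candle whose flame the player can put out.
; Interaction hides the Flame component and sets IsShut when CanBegin is true; otherwise it shows "This candle is out" through the first-person character's NewObjectif.
; ResetAll makes the flame visible again and clears IsShut.
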(event EventResetAll
  (Development|SetHiddeninGame (Variables|Default|Getflame) false false)
  (Variables|Default|SetisShut false))

(event EventInteraction
  (params (CamVector :type Vector :default "0, 0, 0"))
  (if (Variables|Default|GetCanBegin)
    (Development|SetHiddeninGame (Variables|Default|Getflame) true false)
    (Variables|Default|SetisShut true)
    (else
      (bind _asbp_first_person_character (Utilities|Casting|CastToBP_FirstPersonCharacter (Game|GetPlayerCharacter 0)))
      (Default|NewObjectif _asbp_first_person_character "This candle is out" false))))

(fn ConstructionScript)