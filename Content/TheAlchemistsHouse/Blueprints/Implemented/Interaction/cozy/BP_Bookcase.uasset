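; Bookcase puzzle prop that slides aside when the enigma is finished and relays wrong-order resets to its candles.
; EventMove plays a world camera shake at the bookcase, then a timeline lerps the shared root along world X to a hard-coded position.
; WrongOrder, gated by BookTriggered, calls ResetAllMessage on every candle in AllBougie.
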(event Custom|EventMove
  (bind _returnvalue (Transformation|GetActorLocation))
  ;[0.1042 0.1042 0.1042] Deplacement Bookcase fin enigme
  (Camera|PlayWorldCameraShake "/Game/TheAlchemistsHouse/Blueprints/Implemented/UI/BP_CameraShake.BP_CameraShake_C" (Transformation|GetWorldLocation (Variables|Default|GetSharedRoot)) 0.0 1e+03)
  (bind _output_get (Variables|Default|SetInitialLocation (Transformation|GetWorldLocation (Variables|Default|GetSharedRoot))))
  (bind _lerp (Timeline|Movement PlayFromStart)
    (:Update
      (Transformation|SetWorldLocation (Variables|Default|GetSharedRoot) (Math|Vector|MakeVector (Math|Float|Lerp (.x _output_get) -944.0 _lerp) (.y _returnvalue) (.z _returnvalue)) false false))))

(event Custom|WrongOrder
  (if (Variables|Default|GetBookTriggered)
    (for _array_element (Variables|Default|GetAllBougie)
      (Class|BPIInteraction|ResetAll(Message) _array_element))))

(event EventBeginPlay)

(fn ConstructionScript)