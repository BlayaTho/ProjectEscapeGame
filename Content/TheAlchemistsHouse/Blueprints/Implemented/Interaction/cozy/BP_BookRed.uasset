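; BP_BookRed is an interactable red book that is part of a bookcase and candle mechanism.
; Power vision toggles its query collision box and Niagara effect.
; Interaction shows an "already activated" objective if the touched flag is set, otherwise it hits a DoOnce with no follow-up.
; The activation chain that pauses the effect, calls the bookcase's WrongOrder and lets the candle begin is never run.
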(event EventBeginPlay
  (bind _asbp_candle_1 (Utilities|Casting|CastToBP_Candle_1 (Variables|Default|GetCandleREF)))
  (Variables|Default|SetAs%20BP%20Candle%201 _asbp_candle_1)
  (bind _asbp_first_person_character (Utilities|Casting|CastToBP_FirstPersonCharacter (Game|GetPlayerCharacter 0)))
  (Variables|Default|SetAs%20BP%20First%20Person%20Character _asbp_first_person_character))

(event EventPowerVision
  (params (VisionON :type Boolean))
  (bind _ns_bookred (Variables|Default|GetNS_BookRed))
  (bind _box (Variables|Default|GetBox))
  (if VisionON
    (Collision|SetCollisionEnabled _box "QueryOnly")
    (Development|SetHiddeninGame _ns_bookred false false)
    (else
      (Collision|SetCollisionEnabled _box "NoCollision")
      (Development|SetHiddeninGame _ns_bookred true false))))

(event EventInteraction
  (params (CamVector :type Vector :default "0, 0, 0"))
  (if (Variables|Default|GetisAlreadyTouch)
    (Default|NewObjectif (Variables|Default|GetAs%20BP%20First%20Person%20Character) "The mechanism has already been activated" false)
    (else
      (Utilities|FlowControl|DoOnce false))))

(fn ConstructionScript)