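; BP_Candle_4 is an interactable candle in an ordered snuffing puzzle tied to a bookcase.
; Interacting hides its flame and marks it shut only if the preceding BP_Candle_3, referenced through BougieAvant, is already shut.
; Otherwise it reports a wrong answer to the bookcase.
; ResetAll shows the flame again and clears the shut state.
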(event EventResetAll
  (Development|SetHiddeninGame (Variables|Default|GetFlame) false false)
  (Variables|Default|SetisShut false))

(event EventInteraction
  (params (CamVector :type Vector :default "0, 0, 0"))
  (bind _asbp_candle_3 (Utilities|Casting|CastToBP_Candle_3 (Variables|Default|GetBougie%20Avant)))
  (if (Variables|/Game/TheAlchemistsHouse/Blueprints/Implemented/Interaction/cozy/BP_Candle_3.BP_Candle_3_C|GetisShut _asbp_candle_3)
    (Development|SetHiddeninGame (Variables|Default|GetFlame) true false)
    (Variables|Default|SetisShut true)
    (else
      (Default|WrongAnswer (Variables|Default|GetBookcaseRef)))))

(fn ConstructionScript)