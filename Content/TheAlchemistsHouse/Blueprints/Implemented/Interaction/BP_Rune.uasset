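; BP_Rune is a collectible rune that appears and becomes interactable only while power vision is on.
; PowerVision toggles its box query collision and Niagara effect until the rune has been touched.
; A one-time Interaction marks it touched, destroys the linked RuneDoor actor, disables collision, hides the effect and increments the first-person character's NbrRunes1F counter.
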(event EventInteraction
  (params (CamVector :type Vector :default "0, 0, 0"))
  (Utilities|FlowControl|DoOnce false
    (:Completed
      (Variables|Default|SetTouched true)
      (Actor|DestroyActor (Variables|Default|GetRuneDoor))
      (Collision|SetCollisionEnabled (Variables|Default|GetBox) "NoCollision")
      (Development|SetHiddeninGame (Variables|Default|GetNiagara) true false)
      (bind _asbp_first_person_character (Utilities|Casting|CastToBP_FirstPersonCharacter (Game|GetPlayerCharacter 0)))
      (bind _result (Math|Integer|IncrementInt (Variables|/Game/TheAlchemistsHouse/Blueprints/Implemented/Character/BP_FirstPersonCharacter.BP_FirstPersonCharacter_C|GetNbrRunes1F _asbp_first_person_character))
        (:%20%20
          (Variables|/Game/TheAlchemistsHouse/Blueprints/Implemented/Character/BP_FirstPersonCharacter.BP_FirstPersonCharacter_C|SetNbrRunes1F _asbp_first_person_character _result))))))

(event EventPowerVision
  (params (VisionON :type Boolean))
  (if (not (Variables|Default|GetTouched))
    (if VisionON
      (Collision|SetCollisionEnabled (Variables|Default|GetBox) "QueryOnly")
      (Development|SetHiddeninGame (Variables|Default|GetNiagara) false false)
      (else
        (Collision|SetCollisionEnabled (Variables|Default|GetBox) "NoCollision")
        (Development|SetHiddeninGame (Variables|Default|GetNiagara) true false)))))

(fn ConstructionScript)