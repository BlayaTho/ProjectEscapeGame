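; BP_Marmite is an interactable cauldron that reveals a potion once the player has gathered the recipe ingredients.
; BeginPlay caches the first-person character, and Interaction checks its fruit count for exactly four.
; On success, a timeline raises the referenced Potion actor along world Z and sets Finished to block further interaction.
; Otherwise, the character's objective text reports missing ingredients.
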(event EventBeginPlay
  (bind _asbp_first_person_character (Utilities|Casting|CastToBP_FirstPersonCharacter (Game|GetPlayerCharacter 0)))
  (Variables|Default|SetAs%20BP%20First%20Person%20Character _asbp_first_person_character))

(event EventInteraction
  (params (CamVector :type Vector :default "0, 0, 0"))
  (bind _as_bp_first_person_character (Variables|Default|GetAs%20BP%20First%20Person%20Character))
  (bind _potion (Variables|Default|Getpotion))
  (bind _returnvalue (Transformation|GetActorLocation _potion))
  (if (not (Variables|Default|Getfinished))
    (if (== (Variables|/Game/TheAlchemistsHouse/Blueprints/Implemented/Character/BP_FirstPersonCharacter.BP_FirstPersonCharacter_C|GetNbrFruitRecette _as_bp_first_person_character) 4)
      (bind _newtrack_0 (Timeline|TimelineNiagra PlayFromStart)
        (:Update
          (Transformation|SetActorLocation _potion (Math|Vector|MakeVector (.x _returnvalue) (.y _returnvalue) (Math|Float|Lerp 19.0 136.0 _newtrack_0)) false false)
          (Variables|Default|Setfinished true)))
      (else
        (Default|NewObjectif _as_bp_first_person_character "I'm missing some ingredients" false)))))

(fn ConstructionScript)