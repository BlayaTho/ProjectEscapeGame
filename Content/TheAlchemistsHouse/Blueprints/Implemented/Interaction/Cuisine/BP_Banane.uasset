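; BP_Banane is an interactable banana character for a cooking task that comes to life when Ronde runs.
; Ronde shifts its X position, activates it, starts endless random AI roaming through a self-recalling MovementAI, and loops a timed hop.
; A minute later, its walk speed and the pause between moves are changed.
; Interacting increments the player's recipe fruit count and destroys it when active; otherwise, it shows a suspicion message.
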(event Custom|Vitesse
  (Utilities|FlowControl|Delay 6e+01)
  (Variables|/Script/Engine.CharacterMovementComponent|SetMaxWalkSpeed (Variables|Character|GetCharacterMovement) 6e+02)
  (Variables|Default|SetDuration 1.0))

(event Custom|Ronde
  (bind _returnvalue (Transformation|GetActorLocation))
  (Utilities|FlowControl|Sequence
    (:then_0
      (Transformation|SetActorLocation (Math|Vector|MakeVector 613.0 (.y _returnvalue) (.z _returnvalue)) false false)
      (Variables|Default|SetisActive true))
    (:then_1
      (CallFunction|Vitesse))
    (:then_2
      (CallFunction|MovementAI))
    (:then_3
      (Utilities|Time|SetTimerbyEvent (delegate Custom|jumping%20banaa) 1.0 true))))

(event Custom|movementAI
  (AI|AIMoveTo self (.RandomLocation (AI|Navigation|GetRandomReachablePointinRadius (Transformation|GetActorLocation) 1e+04 0 0)) 0 5.0 false
    (:OnSuccess
      (Utilities|FlowControl|Delay (Variables|Default|GetDuration)))
    (:OnFail
      _))
  (CallFunction|MovementAI))

(event Custom|jumping%20banaa
  (Character|Jump)
  (Utilities|FlowControl|Delay 0.5)
  (Character|StopJumping))

(event EventInteraction
  (params (CamVector :type Vector :default "0, 0, 0"))
  (if (Variables|Default|GetisActive)
    (bind _asbp_first_person_character (Utilities|Casting|CastToBP_FirstPersonCharacter (Game|GetPlayerCharacter 0)))
    (bind _result (Math|Integer|IncrementInt (Variables|/Game/TheAlchemistsHouse/Blueprints/Implemented/Character/BP_FirstPersonCharacter.BP_FirstPersonCharacter_C|GetNbrFruitRecette _asbp_first_person_character))
      (:%20%20
        (Variables|/Game/TheAlchemistsHouse/Blueprints/Implemented/Character/BP_FirstPersonCharacter.BP_FirstPersonCharacter_C|SetNbrFruitRecette _asbp_first_person_character _result)
        (Actor|DestroyActor)))
    (else
      (bind _asbp_first_person_character_2 (Utilities|Casting|CastToBP_FirstPersonCharacter (Game|GetPlayerCharacter 0)))
      (Default|NewObjectif _asbp_first_person_character_2 "This banana is very suspicious" false))))

(fn ConstructionScript)