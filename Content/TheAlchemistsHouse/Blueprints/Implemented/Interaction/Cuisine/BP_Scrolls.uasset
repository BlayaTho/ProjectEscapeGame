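; BP_Scrolls is a one-shot trigger in the kitchen (Cuisine) interactions that sets several food actors in motion.
; The first overlap with its Box passes a DoOnce, then starts the apple's teleport, calls Ronde on the banana and sets IsActive on the purple pumpkin and egg.
; These actors come from stored references cast in sequence, so one failed cast skips the remaining activations.
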(event OnComponentBeginOverlap(Box)
  (params (OverlappedComponent :type Primitive%20Component%20Object%20Reference) (OtherActor :type Actor%20Object%20Reference) (OtherComp :type Primitive%20Component%20Object%20Reference) (OtherBodyIndex :type Integer) (bFromSweep :type Boolean) (SweepResult :type Hit%20Result%20Structure%20%28by%20ref%29))
  (Utilities|FlowControl|DoOnce false
    (:Completed
      (bind _asbp_teleport_apple (Utilities|Casting|CastToBP_TeleportApple (Variables|Default|GetBPApple)))
      (Default|DebutTeleport _asbp_teleport_apple)
      (bind _asbp_banane (Utilities|Casting|CastToBP_Banane (Variables|Default|GetBPBanane)))
      (Default|Ronde _asbp_banane)
      (bind _asbp_pumpkin_violet (Utilities|Casting|CastToBP_PumpkinViolet (Variables|Default|GetBPPumpkin)))
      (Variables|/Game/TheAlchemistsHouse/Blueprints/Implemented/Interaction/Cuisine/BP_PumpkinViolet.BP_PumpkinViolet_C|SetisActive _asbp_pumpkin_violet true)
      (bind _asbp_egg (Utilities|Casting|CastToBP_Egg (Variables|Default|GetBPEgg)))
      (Variables|/Game/TheAlchemistsHouse/Blueprints/Implemented/Interaction/Cuisine/BP_Egg.BP_Egg_C|SetisActive _asbp_egg true))))

(fn ConstructionScript)