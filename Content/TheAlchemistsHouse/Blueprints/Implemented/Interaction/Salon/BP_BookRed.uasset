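; BP_BookRed is an interactable red book in the Salon that acts as a trigger for a bookcase mechanism.
; Its first interaction, gated by DoOnce, flags the referenced bookcase as triggered, calls its WrongOrder and shows an objective message on the player character.
; If IsAlreadyTouch is set, interaction only reports the mechanism as already activated.
; PowerVision toggles the book's effect visibility and query-only box collision.
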(event EventBeginPlay
  (bind _asbp_first_person_character (Utilities|Casting|CastToBP_FirstPersonCharacter (Game|GetPlayerCharacter 0)))
  (Variables|Default|SetAs%20BP%20First%20Person%20Character _asbp_first_person_character))

(event EventPowerVision
  (params (VisionON :type Boolean))
  (bind _ns_bookred (Variables|Default|GetNS_BookRed))
  (bind _box (Variables|Default|GetBox))
  (if VisionON
    (Collision|SetCollisionEnabled _box "QueryOnly")
    (Development|SetHiddeninGame _ns_bookred false false)
    (else
      (Collision|SetCollisionEnabled _box "NoCollision")
      (Development|SetHiddeninGame _ns_bookred true false))))

(event EventInteraction
  (params (CamVector :type Vector :default "0, 0, 0"))
  (if (Variables|Default|GetisAlreadyTouch)
    (Default|NewObjectif (Variables|Default|GetAs%20BP%20First%20Person%20Character) "The mechanism has already been activated" false)
    (else
      (Utilities|FlowControl|DoOnce false
        (:Completed
          (Variables|/Game/TheAlchemistsHouse/Blueprints/Implemented/Interaction/BP_Bookcase.BP_Bookcase_C|SetBookTriggered (Variables|Default|GetBookcaseREF) true)
          (Default|WrongOrder (Variables|Default|GetBookcaseREF))
          (Default|NewObjectif (Variables|Default|GetAs%20BP%20First%20Person%20Character) "The book reacted to my presence, a mechanism was activated" false))))))

(fn ConstructionScript)