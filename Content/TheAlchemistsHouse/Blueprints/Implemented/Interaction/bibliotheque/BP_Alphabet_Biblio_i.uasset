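; BP_Alphabet_Biblio_i is an interactable letter I in the library word puzzle of The Alchemist's House.
; On interaction it accepts only if it is untouched and the referenced L letter is already touched, then marks itself touched.
; Otherwise, including a repeat press, it calls WrongWord on the referenced chest.
; ResetAll clears its touched state.
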(event EventInteraction
  (params (CamVector :type Vector :default "0, 0, 0"))
  (if (Variables|Default|GetTouched)
    (Default|WrongWord (Variables|Default|GetChestREF) :!label _label)
    (else
      (bind _asbp_alphabet_biblio_l (Utilities|Casting|CastToBP_Alphabet_Biblio_L (Variables|Default|GetLREF)))
      (if (Variables|/Game/TheAlchemistsHouse/Blueprints/Implemented/Interaction/bibliotheque/BP_Alphabet_Biblio_L.BP_Alphabet_Biblio_L_C|GetTouched _asbp_alphabet_biblio_l)
        (Variables|Default|SetTouched true)
        (else
          (goto _label))))))

(event EventResetAll
  (Variables|Default|SetTouched false))

(fn ConstructionScript)