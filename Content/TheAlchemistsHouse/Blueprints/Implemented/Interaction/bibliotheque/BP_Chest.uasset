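; BP_Chest is a puzzle chest that opens on a correct five-letter combination, or on interaction when flagged as the final chest.
; LetterTouched counts inputs and correctly ordered letters, then either opens the chest or resets the counts and sends a wrong-answer objective to the player.
; A timeline rotates the lid, enabling the key's query collision and moving the bookcase on regular chests.
; The final chest instead reveals a scaling, looping dancing skeletal mesh.
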(event Custom|OpeningchestEvent
  (Utilities|FlowControl|DoOnce false
    (:Completed
      (bind _lerp (Timeline|MovementChest PlayFromStart)
        (:Update
          (Transformation|SetRelativeRotation (Variables|Default|GetChest_cover6_StaticMeshComponent0) (Math|Rotator|MakeRotator (* _lerp (Variables|Default|GetRotationAngle)) 0.0 0.0) false false)
          (if (not (Variables|Default|GetFinalChest))
            (Collision|SetCollisionEnabled (Variables|/Game/TheAlchemistsHouse/Blueprints/Implemented/Interaction/BP_Key.BP_Key_C|GetStaticMesh (Variables|Default|GetKeyY)) "QueryOnly")
            (Default|EventMove (Variables|Default|GetbookcaseREF))))))))

(event Custom|WrongWord
  (bind _as_bp_first_person_character (Variables|Default|GetAs%20BP%20First%20Person%20Character))
  (if (Variables|Default|GetisFirstEventPassed)
    (Default|NewObjectif _as_bp_first_person_character "Wrong answer" true)
    (else
      (Utilities|FlowControl|DoOnce false
        (:Completed
          (Default|NewObjectif _as_bp_first_person_character "A noise tells me it's the wrong combination" false)))))
  (Variables|Default|SetintOrdre 0)
  (Variables|Default|SetintNbrInput 0)
  (Variables|Default|SetisFirstEventPassed true))

(event Custom|LetterTouched
  (params (GoodOrder :type Boolean))
  (bind _result (Math|Integer|IncrementInt (Variables|Default|GetintNbrInput))
    (:%20%20
      (Variables|Default|SetintNbrInput _result)
      (if GoodOrder
        (bind _result_2 (Math|Integer|IncrementInt (Variables|Default|GetintOrdre))
          (:%20%20
            (Variables|Default|SetintOrdre _result_2))))
      (if (== (Variables|Default|GetintNbrInput) 5)
        (if (== (Variables|Default|GetintOrdre) 5)
          (CallFunction|OpeningchestEvent)
          (else
            (CallFunction|WrongWord)))))))

(event Custom|Skeletalanim
  (bind _skeletalmesh (Variables|Default|GetSkeletalMesh))
  (Components|Animation|PlayAnimation (Variables|Default|GetSkeletalMesh) "/Game/TheAlchemistsHouse/SurpriseFin/Northern_Soul_Floor_Combo.Northern_Soul_Floor_Combo" true)
  (bind _lerp (Timeline|Timeline PlayFromStart)
    (:Update
      (Transformation|SetRelativeScale3D _skeletalmesh (Math|Vector|MakeVector (Math|Float|Lerp 0.2 1.6 _lerp) (Math|Float|Lerp 0.2 1.6 _lerp) (Math|Float|Lerp 0.2 1.6 _lerp)))
      (Transformation|SetRelativeLocation _skeletalmesh (Math|Vector|MakeVector 0.0 (Math|Float|Lerp 23.0 125.0 _lerp) 11.0) false false))
    (:Finished
      (Collision|SetActorEnableCollision false))))

(event EventBeginPlay
  (bind _asbp_first_person_character (Utilities|Casting|CastToBP_FirstPersonCharacter (Game|GetPlayerCharacter 0)))
  (Variables|Default|SetAs%20BP%20First%20Person%20Character _asbp_first_person_character))

(event EventInteraction
  (params (CamVector :type Vector :default "0, 0, 0"))
  (if (Variables|Default|GetFinalChest)
    (Utilities|FlowControl|DoOnce false
      (:Completed
        (CallFunction|OpeningchestEvent)
        (Utilities|FlowControl|Delay 1.5)
        (CallFunction|Skeletalanim)))))

(fn ConstructionScript)