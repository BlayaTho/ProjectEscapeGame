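; Library book interactable that works as a one-shot trigger for a linked bookcase, visible to the power vision ability.
; Interaction either scales the linked book stand and closes the bookcase when flagged as the second book, or triggers the bookcase's move event otherwise.
; PowerVision toggles the Niagara effect and enables query-only collision only while active.
; Books flagged non-interactive ignore interaction and collision changes but still show the effect.
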(event EventInteraction
  (params (CamVector :type Vector :default "0, 0, 0"))
  (if (not (Variables|Default|GetisNoInteractif))
    (if (Variables|Default|GetisBook2)
      (Utilities|FlowControl|DoOnce false
        (:Completed
          (bind _asbp_stand_biblio (Utilities|Casting|CastToBP_StandBiblio (Variables|Default|GetstandRef)))
          (Default|ScaleStand _asbp_stand_biblio)
          (Default|CloseBookcase (Variables|Default|GetBookcase2))))
      (else
        (Utilities|FlowControl|DoOnce false
          (:Completed
            (Default|EventMove (Variables|Default|GetBookcase2))))))))

(event EventPowerVision
  (params (VisionON :type Boolean))
  (bind _staticmesh (Variables|Default|GetStaticMesh))
  (if VisionON
    (if (Variables|Default|GetisNoInteractif)
      _
      (else
        (Collision|SetCollisionEnabled _staticmesh "QueryOnly")))
    (Development|SetHiddeninGame (Variables|Default|GetNiagara) false false)
    (else
      (if (Variables|Default|GetisNoInteractif)
        _
        (else
          (Collision|SetCollisionEnabled _staticmesh "NoCollision")))
      (Development|SetHiddeninGame (Variables|Default|GetNiagara) true false))))

(fn ConstructionScript)