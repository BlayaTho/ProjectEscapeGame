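; BP_Alphabet_Biblio_L is the L letter interactable in the library's word puzzle, linked to a chest.
; Interacting marks it Touched only if the referenced A letter is already touched, enforcing spelling order.
; Touching it out of order or a second time calls WrongWord on the chest.
; ResetAll clears its Touched flag.
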(event EventResetAll
  (Variables|Default|SetTouched false))

(event EventInteraction
  (params (CamVector :type Vector :default "0, 0, 0"))
  (if (Variables|Default|GetTouched)
    (Default|WrongWord (Variables|Default|GetChestREF) :!label _label)
    (else
      (bind _asbp_alphabet_biblio_a (Utilities|Casting|CastToBP_Alphabet_Biblio_A (Variables|Default|GetAREF)))
      (if (Variables|/Game/TheAlchemistsHouse/Blueprints/Implemented/Interaction/bibliotheque/BP_Alphabet_Biblio_A.BP_Alphabet_Biblio_A_C|GetTouched _asbp_alphabet_biblio_a)
        (Variables|Default|SetTouched true)
        (else
          (goto _label))))))

(fn ConstructionScript)