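; BP_Bookcase2 is a sliding bookcase in the Alchemist's House library that opens and closes through two events.
; EventMove plays a world camera shake at the bookcase, stores its start location, then runs a Timeline that lerps the root along world X to a hard-coded target.
; CloseBookcase plays the same Timeline in reverse from the end to slide it back, without triggering the shake.
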(event Custom|EventMove
  (bind _returnvalue (Transformation|GetActorLocation))
  (Camera|PlayWorldCameraShake "/Game/TheAlchemistsHouse/Blueprints/Implemented/UI/BP_CameraShake.BP_CameraShake_C" (Transformation|GetWorldLocation (Variables|Default|GetSharedRoot)) 0.0 1e+03)
  (bind _output_get (Variables|Default|SetInitialLocation (Transformation|GetWorldLocation (Variables|Default|GetSharedRoot))))
  (bind _lerp (Timeline|Timeline PlayFromStart)
    (:Update
      (Transformation|SetWorldLocation (Variables|Default|GetSharedRoot) (Math|Vector|MakeVector (Math|Float|Lerp (.x _output_get) -610.2 _lerp) (.y _returnvalue) (.z _returnvalue)) false false))))

(event Custom|CloseBookcase
  (bind _returnvalue (Transformation|GetActorLocation))
  (bind _lerp (Timeline|Timeline ReverseFromEnd)
    (:Update
      (Transformation|SetWorldLocation (Variables|Default|GetSharedRoot) (Math|Vector|MakeVector (Math|Float|Lerp (.x (stale Custom|EventMove _output_get)) -610.2 _lerp) (.y _returnvalue) (.z _returnvalue)) false false))))

(fn ConstructionScript)