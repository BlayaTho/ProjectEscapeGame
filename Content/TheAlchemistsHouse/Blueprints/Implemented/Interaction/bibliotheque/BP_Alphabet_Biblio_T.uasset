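; BP_Alphabet_Biblio_T is the "T" letter interactable in the library alphabet puzzle of The Alchemist's House, closing the word sequence.
; On interaction it checks that the linked O letter was touched, then once triggers the chest opening and the bookcase movement.
; If O was not touched it signals a wrong word to the chest, and ResetAll clears its Touched state.
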(event EventResetAll
  (Variables|Default|SetTouched false))

(event EventInteraction
  (params (CamVector :type Vector :default "0, 0, 0"))
  (bind _chestref (Variables|Default|GetChestREF))
  (bind _asbp_alphabet_biblio_o (Utilities|Casting|CastToBP_Alphabet_Biblio_O (Variables|Default|GetOREF)))
  (if (Variables|/Game/TheAlchemistsHouse/Blueprints/Implemented/Interaction/bibliotheque/BP_Alphabet_Biblio_O.BP_Alphabet_Biblio_O_C|GetTouched _asbp_alphabet_biblio_o)
    (Utilities|FlowControl|DoOnce false
      (:Completed
        (Default|OpeningchestEvent _chestref)
        (Default|EventMove (Variables|Default|GetBookcaseREF))))
    (else
      (Default|WrongWord _chestref))))

(fn ConstructionScript)