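; BP_Bookcase is the candle puzzle's bookcase that slides aside when the puzzle is solved.
; It gathers every BP_Candle at BeginPlay and counts touches, opening on the sixth.
; A wrong order, while BookTriggered is set, zeroes the count and resets all candles.
; Opening plays a camera shake and a timeline that lerps the root along X, which CloseBookcase plays in reverse.
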(event Custom|EventMove
  (bind _returnvalue (Transformation|GetActorLocation))
  ;[0.1042 0.1042 0.1042] Deplacement Bookcase fin enigme
  (Camera|PlayWorldCameraShake "/Game/TheAlchemistsHouse/Blueprints/Implemented/UI/BP_CameraShake.BP_CameraShake_C" (Transformation|GetWorldLocation (Variables|Default|GetSharedRoot)) 0.0 7e+02)
  (bind _output_get (Variables|Default|SetInitialLocation (Transformation|GetWorldLocation (Variables|Default|GetSharedRoot))))
  (bind _lerp (Timeline|Movement PlayFromStart)
    (:Update
      (Transformation|SetWorldLocation (Variables|Default|GetSharedRoot) (Math|Vector|MakeVector (Math|Float|Lerp (.x _output_get) (Variables|Default|GetDestinationX) _lerp) (.y _returnvalue) (.z _returnvalue)) false false))))

(event Custom|WrongOrder
  ;[1 1 1] Enigme Bougie
  (if (Variables|Default|GetBookTriggered)
    (Variables|Default|SetintOrdre 0)
    (for _array_element (Variables|Default|GetAllBougie)
      (Class|BPIInteraction|ResetAll(Message) _array_element))))

(event Custom|BougieToucher
  ;[1 1 1] Enigme Bougie
  (bind _result (Math|Integer|IncrementInt (Variables|Default|GetintOrdre))
    (:%20%20
      (Variables|Default|SetintOrdre _result)
      (if (== (Variables|Default|GetintOrdre) 6)
        (CallFunction|EventMove)))))

(event Custom|CloseBookcase
  (bind _returnvalue (Transformation|GetActorLocation))
  ;[0.1042 0.1042 0.1042] Deplacement Bookcase fin enigme
  (bind _lerp (Timeline|Movement ReverseFromEnd)
    (:Update
      (Transformation|SetWorldLocation (Variables|Default|GetSharedRoot) (Math|Vector|MakeVector (Math|Float|Lerp (.x (stale Custom|EventMove _output_get)) (Variables|Default|GetDestinationX) _lerp) (.y _returnvalue) (.z _returnvalue)) false false))))

(event EventBeginPlay
  ;[1 1 1] Enigme Bougie
  (bind _outactors (Actor|GetAllActorsOfClass "/Game/TheAlchemistsHouse/Blueprints/Implemented/Interaction/Salon/BP_Candle.BP_Candle_C"))
  (for _array_element _outactors
    (Utilities|Array|Add (Variables|Default|GetAllBougie) _array_element)))

(fn ConstructionScript)