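; Interactable double door that can be locked by a green or yellow key, or blocked entirely with an objective message.
; Interaction checks the player character's key flags, showing a message if the key is missing or destroying the Niagara symbol actor if held.
; A FlipFlop plays or reverses a duration-scaled timeline rotating both leaves oppositely, with swing direction set by comparing camera vector to doorway right vector.
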(event EventBeginPlay
  (Components|Timeline|SetPlayRate (Variables|Default|GetMovementDoor) (/ 1.0 (Variables|OpeningSystem|GetDuration)))
  (bind _asbp_first_person_character (Utilities|Casting|CastToBP_FirstPersonCharacter (Game|GetPlayerCharacter 0)))
  (Variables|Default|SetAs%20BP%20First%20Person%20Character _asbp_first_person_character))

(event EventInteraction
  (params (CamVector :type Vector :default "0, 0, 0"))
  (bind _as_bp_first_person_character (Variables|Default|GetAs%20BP%20First%20Person%20Character))
  (bind _as_bp_first_person_character_2 (Variables|Default|GetAs%20BP%20First%20Person%20Character))
  (if (Variables|OpeningSystem|GetCanOpen)
    (if (Variables|OpeningSystem|GetNeedGreen)
      (if (Variables|/Game/TheAlchemistsHouse/Blueprints/Implemented/Character/BP_FirstPersonCharacter.BP_FirstPersonCharacter_C|GetKeyG _as_bp_first_person_character_2)
        (Actor|DestroyActor (Variables|Default|GetniagaraSymbol))
        (if (not (Variables|Default|GetIsOpening)) :!label _label
          (if (Variables|Default|GetIsOpen)
            _
            (elif (Utilities|Operators|EqualEqual CamVector (Math|Vector|GetRightVector (Variables|Default|GetSM_Door_aperture)) 1.0)
              (Variables|OpeningSystem|SetRotationAngle (* (Variables|OpeningSystem|GetRotationAngle) -1.0))
              (else
                (Variables|OpeningSystem|SetRotationAngle (Math|Float|Absolute(Float) (Variables|OpeningSystem|GetRotationAngle))))))
          (Utilities|FlowControl|FlipFlop
            (:A
              (Variables|Default|SetIsOpening true)
              (Variables|Default|SetIsOpen true)
              (bind _newtrack_0 (Timeline|MovementDoor Play)
                (:Update
                  (Transformation|SetRelativeRotation (Variables|Default|GetSM_DoorL) (Math|Rotator|MakeRotator 0.0 0.0 (* (* _newtrack_0 (Variables|OpeningSystem|GetRotationAngle)) -1.0)) false false)
                  (Transformation|SetRelativeRotation (Variables|Default|GetSM_DoorR) (Math|Rotator|MakeRotator 0.0 0.0 (* _newtrack_0 (Variables|OpeningSystem|GetRotationAngle))) false false)
                  (Variables|Default|SetIsOpening false))))
            (:B
              (Variables|Default|SetIsOpening true)
              (Variables|Default|SetIsOpen false)
              (Timeline|MovementDoor Reverse))))
        (else
          (Default|NewObjectif _as_bp_first_person_character_2 "I need a key to open this door" false)))
      (elif (Variables|OpeningSystem|GetNeedYellow)
        (if (Variables|/Game/TheAlchemistsHouse/Blueprints/Implemented/Character/BP_FirstPersonCharacter.BP_FirstPersonCharacter_C|GetKeyY _as_bp_first_person_character)
          (Actor|DestroyActor (Variables|Default|GetniagaraSymbol))
          (goto _label)
          (else
            (Default|NewObjectif _as_bp_first_person_character "I need a yellow key to open this door" false)))
        (else
          (goto _label))))
    (else
      (Default|NewObjectif (Variables|Default|GetAs%20BP%20First%20Person%20Character) "That's the door I came from" false))))

(fn ConstructionScript)